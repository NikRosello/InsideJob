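; BP_CLUE is a collectible clue actor that the player picks up through an Interact event.
; On interaction it hides and disables collision on its mesh, then shows a WBP_ClueFound widget for a one-second delay.
; It then removes the widget, increments ClueCount on the third-person player character, prints the new count and destroys itself.
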(event `/Game/Input/BPI_Interact.Interact`
  (params (HoldPoint :type "SceneComponent Object Reference"))
  (`SceneComponent.SetHiddenInGame` (`self.CLUEMesh`) true false)
  (`PrimitiveComponent.SetCollisionEnabled` (`self.CLUEMesh`) "NoCollision")
  (bind _returnvalue (`|CreateWidget` "/Game/WBP_ClueFound.WBP_ClueFound_C"))
  (`UserWidget.AddToViewport` _returnvalue 0)
  (`KismetSystemLibrary.Delay` 1.0)
  (`Widget.RemoveFromParent` _returnvalue)
  (bind _asbp_third_person_character (cast `/Game/ThirdPerson/Blueprints/BP_ThirdPersonCharacter` (`GameplayStatics.GetPlayerCharacter` 0)))
  (set `/Game/ThirdPerson/Blueprints/BP_ThirdPersonCharacter.ClueCount` (+ (`/Game/ThirdPerson/Blueprints/BP_ThirdPersonCharacter.ClueCount` _asbp_third_person_character) 1) _asbp_third_person_character)
  (`KismetSystemLibrary.PrintString` (`KismetStringLibrary.Conv_IntToString` (`/Game/ThirdPerson/Blueprints/BP_ThirdPersonCharacter.ClueCount` _asbp_third_person_character)))
  (`self.K2_DestroyActor`))

(fn `UserConstructionScript`)