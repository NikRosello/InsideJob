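; Turret actor that tracks the player and shoots bullets while the third-person character is within range.
; DetectionRadius overlap events toggle InRange, which lets Tick rotate BaseTurret toward player 0 using a look-at rotation.
; BeginPlay starts a looping one-second timer, and Fire spawns Bp_TurretBullets at the Gun transform when InRange is set.
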(event `self.ReceiveTick`
  (params (DeltaSeconds :type "Float (single-precision)"))
  (if (`self.InRange`)
    (`SceneComponent.K2_SetWorldRotation` (`self.BaseTurret`) (`KismetMathLibrary.FindLookAtRotation` (`self.K2_GetActorLocation`) (`self.K2_GetActorLocation` (`GameplayStatics.GetPlayerCharacter` 0))) false false)))

(event `self.DetectionRadius.OnComponentBeginOverlap`
  (params (OverlappedComponent :type "PrimitiveComponent Object Reference") (OtherActor :type "Actor Object Reference") (OtherComp :type "PrimitiveComponent Object Reference") (OtherBodyIndex :type Integer) (bFromSweep :type Boolean) (SweepResult :type "HitResult Structure (by ref)"))
  (cast `/Game/ThirdPerson/Blueprints/BP_ThirdPersonCharacter` OtherActor)
  (set `self.InRange` true))

(event `self.DetectionRadius.OnComponentEndOverlap`
  (params (OverlappedComponent :type "PrimitiveComponent Object Reference") (OtherActor :type "Actor Object Reference") (OtherComp :type "PrimitiveComponent Object Reference") (OtherBodyIndex :type Integer))
  (cast `/Game/ThirdPerson/Blueprints/BP_ThirdPersonCharacter` OtherActor)
  (set `self.InRange` false))

(event `self.ReceiveBeginPlay`
  (`KismetSystemLibrary.K2_SetTimerDelegate` (`|CreateDelegate` :!event `fire`) 1.0 true))

(fn `fire`
  (if (`self.InRange`)
    (`|SpawnActorFromClass` "/Game/Blueprints/bp_TurretBullets.bp_TurretBullets_C" (`SceneComponent.K2_GetComponentToWorld` (`self.Gun`)) "Undefined" "MultiplyWithRoot" null null)))

(fn `UserConstructionScript`)