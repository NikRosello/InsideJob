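; Bp_Button is a color-keyed pressure button that reports its pressed state to a linked door.
; Actors tagged with the ButtonColor value set IsPressed when they enter the trigger and clear it when they leave, each time calling ButtonsChecked on TargetDoor.
; A timeline plays and reverses to lerp the button mesh down and back up between positions cached at BeginPlay.
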(event `self.ReceiveBeginPlay`
  (bind _output_get (set `self.ButtonStart` (`SceneComponent.RelativeLocation` (`self.Button`))))
  (bind _output_get_2 (set `self.ButtonPressed` (+ (`SceneComponent.RelativeLocation` (`self.Button`)) (0.0 0.0 -15.0)))))

(event `self.Trigger.OnComponentBeginOverlap`
  (params (OverlappedComponent :type "PrimitiveComponent Object Reference") (OtherActor :type "Actor Object Reference") (OtherComp :type "PrimitiveComponent Object Reference") (OtherBodyIndex :type Integer) (bFromSweep :type Boolean) (SweepResult :type "HitResult Structure (by ref)"))
  (if (`self.ActorHasTag` OtherActor (`self.ButtonColor`))
    (set `self.IsPressed` true)
    (`/Game/Doors/Bp_Door.ButtonsChecked` (`self.TargetDoor`))
    (bind (_direction _alpha) (`Timeline|ButtonDown` :!label _label)
      (:`Update`
        (`SceneComponent.K2_SetRelativeLocation` (`self.Button`) (`KismetMathLibrary.VLerp` (stale `self.ReceiveBeginPlay` _output_get) (stale `self.ReceiveBeginPlay` _output_get_2) _alpha) false true)))))

(event `self.Trigger.OnComponentEndOverlap`
  (params (OverlappedComponent :type "PrimitiveComponent Object Reference") (OtherActor :type "Actor Object Reference") (OtherComp :type "PrimitiveComponent Object Reference") (OtherBodyIndex :type Integer))
  (if (`self.ActorHasTag` OtherActor (`self.ButtonColor`))
    (set `self.IsPressed` false)
    (`/Game/Doors/Bp_Door.ButtonsChecked` (`self.TargetDoor`))
    (goto _label :!via `Reverse`)))

(fn `UserConstructionScript`)