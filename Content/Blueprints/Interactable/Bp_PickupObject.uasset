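; Interactable pickup object that the player can grab and release through an Interact event.
; A Holding flag toggles each call between picking up and dropping.
; Pickup turns off the static mesh's physics and collision, then snaps it to the supplied HoldPoint component.
; Release detaches it at its current world transform and restores collision and physics simulation.
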(event `/Game/Input/BPI_Interact.Interact`
  (params (HoldPoint :type "SceneComponent Object Reference"))
  (if (`self.Holding`)
    (set `self.Holding` false)
    (`self.K2_DetachFromActor` "KeepWorld" "KeepWorld" "KeepWorld")
    (`PrimitiveComponent.SetCollisionEnabled` (`self.StaticMesh`) "QueryAndPhysics")
    (`PrimitiveComponent.SetSimulatePhysics` (`self.StaticMesh`) true)
    (else
      (set `self.Holding` true)
      (`PrimitiveComponent.SetSimulatePhysics` (`self.StaticMesh`) false)
      (`PrimitiveComponent.SetCollisionEnabled` (`self.StaticMesh`) "NoCollision")
      (`self.K2_AttachToComponent` HoldPoint "None" "SnapToTarget" "SnapToTarget" "SnapToTarget" false))))

(fn `UserConstructionScript`)