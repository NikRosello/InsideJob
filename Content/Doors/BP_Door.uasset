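; BP_Door is a door that rotates on its pivot, driven by interaction or by a three-button check.
; Interact plays or reverses the TL_Door timeline depending on DoorOpen, animating the pivot's yaw.
; ButtonsChecked snaps the pivot open and sets DoorOpen when the red, blue and green buttons are all pressed, otherwise snapping it closed and clearing the flag.
; Interact itself never changes DoorOpen.
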(event `/Game/Input/BPI_Interact.Interact`
  (params (HoldPoint :type "SceneComponent Object Reference"))
  (if (`self.DoorOpen`)
    (bind (_direction _moving) (`Timeline|TL_Door` :!via `Reverse` :!label _label)
      (:`Update`
        (`SceneComponent.K2_SetRelativeRotation` (`self.DoorPivot`) (`KismetMathLibrary.MakeRotator` 0.0 0.0 _moving) false false)))
    (else
      (goto _label))))

(fn `ButtonsChecked`
  (if (and (and (`/Game/Blueprints/Interactable/Bp_Button.IsPressed` (`self.RedButton`)) (`/Game/Blueprints/Interactable/Bp_Button.IsPressed` (`self.BlueButton`))) (`/Game/Blueprints/Interactable/Bp_Button.IsPressed` (`self.GreenButton`)))
    (`SceneComponent.K2_SetRelativeRotation` (`self.DoorPivot`) (struct :`Yaw` -90.0) false false)
    (set `self.DoorOpen` true)
    (else
      (`SceneComponent.K2_SetRelativeRotation` (`self.DoorPivot`) (struct) false false)
      (set `self.DoorOpen` false))))

(fn `UserConstructionScript`)