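; Interactable hinged main door that toggles open and closed, picking its swing direction from the side the player is on.
; Front and back trigger overlaps with the third-person character record that side, which sets a positive or negative 90-degree yaw target on opening.
; A timeline scales that angle to rotate the door pivot, playing to open and reversing to close.
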(event `self.Interact`
  (params (HoldPoint :type "SceneComponent Object Reference"))
  (if (`self.Door Open`)
    (set `self.Door Open` false)
    (bind (_direction _dooralpha) (`Timeline|TL_Door` :!via `Reverse` :!label _label)
      (:`Update`
        (`SceneComponent.K2_SetRelativeRotation` (`self.DoorPivot`) (`KismetMathLibrary.MakeRotator` 0.0 0.0 (* _dooralpha (`self.Open Direction`))) false false)))
    (elif (`self.Player Front`)
      (set `self.Open Direction` -90.0)
      (set `self.Door Open` true)
      (goto _label)
      (else
        (set `self.Open Direction` 90.0)
        (set `self.Door Open` true)
        (goto _label)))))

(event `self.FrontT.OnComponentBeginOverlap`
  (params (OverlappedComponent :type "PrimitiveComponent Object Reference") (OtherActor :type "Actor Object Reference") (OtherComp :type "PrimitiveComponent Object Reference") (OtherBodyIndex :type Integer) (bFromSweep :type Boolean) (SweepResult :type "HitResult Structure (by ref)"))
  (cast `/Game/ThirdPerson/Blueprints/BP_ThirdPersonCharacter` OtherActor)
  (set `self.Player Front` true))

(event `self.BackT.OnComponentBeginOverlap`
  (params (OverlappedComponent :type "PrimitiveComponent Object Reference") (OtherActor :type "Actor Object Reference") (OtherComp :type "PrimitiveComponent Object Reference") (OtherBodyIndex :type Integer) (bFromSweep :type Boolean) (SweepResult :type "HitResult Structure (by ref)"))
  (cast `/Game/ThirdPerson/Blueprints/BP_ThirdPersonCharacter` OtherActor)
  (set `self.Player Front` false))

(fn `UserConstructionScript`)